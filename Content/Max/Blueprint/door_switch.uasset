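; Sliding door that starts locked or unlocked, shown by a red or green point light, and can be unlocked by a linked switch.
; The switch's pressed event clears the lock and updates the light color, which the construction script also sets.
; The player entering the box enables Interact input, which plays the slide timeline if unlocked.
; End overlap disables input and reverses the timeline only for AI_Statue actors.
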(event OnComponentBeginOverlap(Box)
  (params (OverlappedComponent :type Primitive%20Component%20Object%20Reference) (OtherActor :type Actor%20Object%20Reference) (OtherComp :type Primitive%20Component%20Object%20Reference) (OtherBodyIndex :type Integer) (bFromSweep :type Boolean) (SweepResult :type Hit%20Result%20Structure%20%28by%20ref%29))
  (Utilities|Casting|CastToFirstPersonCharacter OtherActor)
  (Input|EnableInput (Game|GetPlayerController 0)))

(event OnComponentEndOverlap(Box)
  (params (OverlappedComponent :type Primitive%20Component%20Object%20Reference) (OtherActor :type Actor%20Object%20Reference) (OtherComp :type Primitive%20Component%20Object%20Reference) (OtherBodyIndex :type Integer))
  (Utilities|Casting|CastToAI_Statue OtherActor)
  (Input|DisableInput (Game|GetPlayerController 0))
  (bind _doorsliding (Timeline|Door%20Animation Reverse)
    (:Update
      (Transformation|SetRelativeLocation (Variables|Default|GetDoorMesh) _doorsliding false false))))

(event Custom|UnlockDoor
  (params (Switch :type Switch%20Object%20Reference))
  (bind _pointlight (Variables|Default|GetPointLight))
  (if (== Switch (Variables|Default|GetSwitch))
    (bind _output_get (Variables|Default|SetIsLocked false))
    (if _output_get
      (Rendering|Components|Light|SetLightColor _pointlight "(R=1.000000,G=0.000000,B=0.000000,A=1.000000)" true)
      (else
        (Rendering|Components|Light|SetLightColor _pointlight "(R=0.023159,G=1.000000,B=0.000000,A=1.000000)" true)))))

(event EventBeginPlay
  (EventDispatchers|BindEventtoSwitchPressed (Variables|Default|GetSwitch) (delegate Custom|UnlockDoor)))

(event Input|ActionEvents|InputActionInteract
  (params (Key :type Key%20Structure :default "None"))
  (:Pressed
    (if (not (Variables|Default|GetIsLocked))
      (bind _doorsliding (Timeline|Door%20Animation Play)
        (:Update
          (Transformation|SetRelativeLocation (Variables|Default|GetDoorMesh) _doorsliding false false))))))

(fn ConstructionScript
  (bind _pointlight (Variables|Default|GetPointLight))
  (if (Variables|Default|GetIsLocked)
    (Rendering|Components|Light|SetLightColor _pointlight "(R=1.000000,G=0.000000,B=0.000000,A=1.000000)" true)
    (else
      (Rendering|Components|Light|SetLightColor _pointlight "(R=0.023159,G=1.000000,B=0.000000,A=1.000000)" true))))