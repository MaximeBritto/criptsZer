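; Light puzzle piece that acts on the BP_pad it is attached to as a child actor.
; Its test event first uses a DoOnce to cache the parent pad and its Cube mesh.
; It then calls UpdatePads on that pad whenever CanChangeMat is true.
; The cached mesh is not used elsewhere in this graph.
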(event Custom|test
  (Utilities|FlowControl|Sequence
    (:then_0
      (Utilities|FlowControl|DoOnce false
        (:Completed
          (bind _asbp_pad (Utilities|Casting|CastToBP_pad (Actor|GetParentActor)))
          (Variables|Default|SetparentActor _asbp_pad)
          (Variables|Default|SetparentStaticMesh (Variables|/Game/Julien/Enigma/BP_pad.BP_pad_C|GetCube _asbp_pad)))))
    (:then_1
      (if (Variables|/Game/Julien/Enigma/BP_pad.BP_pad_C|GetcanChangeMat? (Variables|Default|GetparentActor))
        (Default|UpdatePads (Variables|Default|GetparentActor))))))

(fn ConstructionScript)