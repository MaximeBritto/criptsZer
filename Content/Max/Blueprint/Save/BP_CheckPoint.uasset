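; Checkpoint trigger actor that saves the first-person player's position and restores it when play begins.
; Overlapping its Box loads or creates a checkpoint_savegame, writes the character's current location into it and saves it to the single "CheckPointSlot" slot.
; On BeginPlay, each instance loads that slot and, if the save is valid, teleports player pawn 0 to the stored location with zeroed rotation.
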(event OnComponentBeginOverlap(Box)
  (params (OverlappedComponent :type Primitive%20Component%20Object%20Reference) (OtherActor :type Actor%20Object%20Reference) (OtherComp :type Primitive%20Component%20Object%20Reference) (OtherBodyIndex :type Integer) (bFromSweep :type Boolean) (SweepResult :type Hit%20Result%20Structure%20%28by%20ref%29))
  (bind _asfirst_person_character (Utilities|Casting|CastToFirstPersonCharacter OtherActor))
  (Development|PrintString "Hello")
  (Variables|Default|Setlocation (Transformation|GetActorLocation _asfirst_person_character))
  (bind _returnvalue (SaveGame|DoesSaveGameExist "CheckPointSlot"))
  (if _returnvalue
    (bind _returnvalue_2 (SaveGame|LoadGamefromSlot "CheckPointSlot"))
    (bind _output_get (Variables|Default|Setsavesubclass _returnvalue_2))
    (bind _ascheckpoint_savegame (Utilities|Casting|CastTocheckpoint_savegame _output_get))
    (Variables|/Game/Max/Blueprint/Save/checkpoint_savegame.checkpoint_savegame_C|SetoneLocation _ascheckpoint_savegame (Variables|Default|Getlocation))
    (SaveGame|SaveGametoSlot (Variables|Default|Getsavesubclass) "CheckPointSlot")
    (else
      (bind _returnvalue_3 (SaveGame|CreateSaveGameObject "/Game/Max/Blueprint/Save/checkpoint_savegame.checkpoint_savegame_C"))
      (bind _output_get_2 (Variables|Default|Setsavesubclass _returnvalue_3))
      (bind _ascheckpoint_savegame_2 (Utilities|Casting|CastTocheckpoint_savegame _output_get_2))
      (Variables|/Game/Max/Blueprint/Save/checkpoint_savegame.checkpoint_savegame_C|SetoneLocation _ascheckpoint_savegame_2 (Variables|Default|Getlocation))
      (SaveGame|SaveGametoSlot (Variables|Default|Getsavesubclass) "CheckPointSlot"))))

(event EventBeginPlay
  (bind _returnvalue (SaveGame|LoadGamefromSlot "CheckPointSlot"))
  (bind _output_get (Variables|Default|Setsavesubclass _returnvalue))
  (bind _ascheckpoint_savegame (Utilities|Casting|CastTocheckpoint_savegame _output_get))
  (Transformation|Teleport (Game|Player|GetPlayerPawn 0) (Variables|/Game/Max/Blueprint/Save/checkpoint_savegame.checkpoint_savegame_C|GetoneLocation _ascheckpoint_savegame) "0, 0, 0"))

(fn ConstructionScript)