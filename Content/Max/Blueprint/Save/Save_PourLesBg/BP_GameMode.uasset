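; Game mode that saves and restores the first-person character's transform through a single save slot.
; BeginPlay creates the save if none exists, otherwise moves the player to the saved transform when the save's UseSaveLocaTion flag is set.
; SaveGame writes the current transform to the slot.
; LoadGame restarts the level so BeginPlay reapplies it, while RestartLevel deletes the save before restarting.
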(event Custom|SaveGame
  ;[1 1 1] Save Game
  (bind _returnvalue (SaveGame|LoadGamefromSlot "save1"))
  (bind _asbp_save_game_zer (Utilities|Casting|CastToBp_SaveGameZer _returnvalue))
  (Variables|/Game/Max/Blueprint/Save/Save_PourLesBg/Bp_SaveGameZer.Bp_SaveGameZer_C|SetcharTransform _asbp_save_game_zer (Transformation|GetActorTransform (.AsFirst%20Person%20Character (Utilities|Casting|CastToFirstPersonCharacter (Game|GetPlayerCharacter 0)))))
  (SaveGame|SaveGametoSlot _asbp_save_game_zer "save1"))

(event Custom|LoadGame
  (Development|ExecuteConsoleCommand "RestartLevel" 0))

(event Custom|RestartLevel
  (SaveGame|DeleteGameinSlot "save1")
  (Development|ExecuteConsoleCommand "RestartLevel" 0))

(event EventBeginPlay
  (bind _returnvalue (SaveGame|DoesSaveGameExist "save1"))
  (if _returnvalue
    (bind _returnvalue_2 (SaveGame|LoadGamefromSlot "save1"))
    (bind _asbp_save_game_zer (Utilities|Casting|CastToBp_SaveGameZer _returnvalue_2))
    (if (Variables|/Game/Max/Blueprint/Save/Save_PourLesBg/Bp_SaveGameZer.Bp_SaveGameZer_C|GetUseSaveLocaTion _asbp_save_game_zer)
      ;[1 1 1] Load game fonctionality
      (bind _asfirst_person_character (Utilities|Casting|CastToFirstPersonCharacter (Game|GetPlayerCharacter 0)))
      (Transformation|SetWorldTransform (Variables|/Script/Engine.Actor|GetRootComponent _asfirst_person_character) (Variables|/Game/Max/Blueprint/Save/Save_PourLesBg/Bp_SaveGameZer.Bp_SaveGameZer_C|GetcharTransform _asbp_save_game_zer) false false))
    (else
      ;[1 1 1] Save File Create
      (bind _returnvalue_3 (SaveGame|CreateSaveGameObject "/Game/Max/Blueprint/Save/Save_PourLesBg/Bp_SaveGameZer.Bp_SaveGameZer_C"))
      (SaveGame|SaveGametoSlot _returnvalue_3 "save1"))))

(fn ConstructionScript)