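; BP_door is a door that rotates its static mesh open and closed through the OpenDoor and CloseDoor events.
; BeginPlay caches the mesh's world rotation as the default.
; OpenDoor plays a timeline whose ZAxis track supplies a yaw offset combined with that default each update, and CloseDoor reverses the same timeline.
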(event Custom|OpenDoor
  (bind _zaxis (Timeline|DoorTimeLine Play)
    (:Update
      (Transformation|SetWorldRotation (Variables|Debug|GetStaticMeshComponent) (Math|Rotator|CombineRotators (Math|Rotator|MakeRotator 0.0 0.0 _zaxis) (Variables|Default|GetDefaultRotation)) false false))))

(event Custom|CloseDoor
  (bind _zaxis (Timeline|DoorTimeLine Reverse)
    (:Update
      (Transformation|SetWorldRotation (Variables|Debug|GetStaticMeshComponent) (Math|Rotator|CombineRotators (Math|Rotator|MakeRotator 0.0 0.0 _zaxis) (Variables|Default|GetDefaultRotation)) false false))))

(event EventBeginPlay
  (Variables|Default|SetDefaultRotation (Transformation|GetWorldRotation (Variables|Debug|GetStaticMeshComponent))))

(fn ConstructionScript)