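; Readable note Blueprint that shows an interact prompt widget while the first-person character is inside its box trigger.
; The Interact input drives a FlipFlop that alternately opens and closes the note widget, briefly flagging the prompt as pressed.
; A first-enter flag, set on leaving the box, routes the closing branch to opening instead.
; Leaving the box removes both the prompt and any open note.
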(event OnComponentBeginOverlap(Box)
  (params (OverlappedComponent :type Primitive%20Component%20Object%20Reference) (OtherActor :type Actor%20Object%20Reference) (OtherComp :type Primitive%20Component%20Object%20Reference) (OtherBodyIndex :type Integer) (bFromSweep :type Boolean) (SweepResult :type Hit%20Result%20Structure%20%28by%20ref%29))
  (Utilities|Casting|CastToFirstPersonCharacter OtherActor)
  (if (not (Variables|Default|GetalreadyAddToViewport))
    (bind _returnvalue (UserInterface|CreateWidget "/Game/Julien/UI/Door/Interact.Interact_C"))
    (UserInterface|Viewport|AddtoViewport _returnvalue 0)
    (Variables|Default|SetalreadyAddToViewport true)))

(event OnComponentEndOverlap(Box)
  (params (OverlappedComponent :type Primitive%20Component%20Object%20Reference) (OtherActor :type Actor%20Object%20Reference) (OtherComp :type Primitive%20Component%20Object%20Reference) (OtherBodyIndex :type Integer))
  (Utilities|Casting|CastToFirstPersonCharacter OtherActor)
  (Widget|RemovefromParent (stale OnComponentBeginOverlap(Box) _returnvalue))
  (Variables|Default|SetalreadyAddToViewport false)
  (Variables|Default|SetfirstEnterTrigger true)
  (if (Variables|Default|GetcanSeeNote?)
    (Widget|RemovefromParent (stale Input|ActionEvents|InputActionInteract _returnvalue))
    (Variables|Default|SetcanSeeNote? false)))

(event EventBeginPlay
  (Input|EnableInput (Game|GetPlayerController 0)))

(event Input|ActionEvents|InputActionInteract
  (params (Key :type Key%20Structure :default "None"))
  (:Pressed
    (Utilities|FlowControl|FlipFlop
      (:A
        (if (Variables|Default|GetalreadyAddToViewport)
          (if (Variables|Default|GetfirstEnterTrigger)
            _
            (else
              _))
          (Variables|/Game/Julien/UI/Door/Interact.Interact_C|SetisPressed (stale OnComponentBeginOverlap(Box) _returnvalue) true :!label _label)
          (Utilities|FlowControl|Delay 0.2)
          (Variables|/Game/Julien/UI/Door/Interact.Interact_C|SetisPressed (stale OnComponentBeginOverlap(Box) _returnvalue) false)
          (Variables|Default|SetfirstEnterTrigger false)
          (if (not (Variables|Default|GetcanSeeNote?))
            (bind _returnvalue (UserInterface|CreateWidget "/Game/Max/Blueprint/Note_Bp/WG_Note.WG_Note_C"))
            (UserInterface|Viewport|AddtoViewport _returnvalue 0)
            (Variables|Default|SetcanSeeNote? true))))
      (:B
        (if (Variables|Default|GetalreadyAddToViewport)
          (if (Variables|Default|GetfirstEnterTrigger)
            (goto _label)
            (else
              (Variables|/Game/Julien/UI/Door/Interact.Interact_C|SetisPressed (stale OnComponentBeginOverlap(Box) _returnvalue) true)
              (Utilities|FlowControl|Delay 0.2)
              (Variables|/Game/Julien/UI/Door/Interact.Interact_C|SetisPressed (stale OnComponentBeginOverlap(Box) _returnvalue) false)
              (if (Variables|Default|GetcanSeeNote?)
                (Widget|RemovefromParent _returnvalue)
                (Variables|Default|SetcanSeeNote? false)))))))))

(fn ConstructionScript)