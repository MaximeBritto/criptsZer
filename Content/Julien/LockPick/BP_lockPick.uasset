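; BP_lockPick is an unfinished lockpicking actor with a bobby pin and a scene capture that renders only the actor's own components.
; Input axes store the lock turn value and check whether pin rotation is allowed, which requires zero lock input and enabled tick.
; That check drives nothing yet, RotatePin only zeroes the pin's rotation with its clamp unused, and most lock, unlock-range and tick functions are empty stubs.
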(event Input|AxisEvents|InputAxisRotatePin
  (params (AxisValue :type Float%20%28single-precision%29))
  (Utilities|AllowedPinRotation))

(event Input|AxisEvents|InputAxisRotateLock
  (params (AxisValue :type Float%20%28single-precision%29))
  (Variables|Private|SetRotateLockAxis AxisValue))

(fn ConstructionScript
  (Rendering|SceneCapture|ShowOnlyActorComponents (Variables|Default|GetSceneCaptureComponent2D) self false))

(fn GetLockRotation)

(fn GetPinRotation
  (return (.roll (Variables|/Script/Engine.SceneComponent|GetRelativeRotation (Variables|Default|GetbobbyPin)))))

(fn IsPininUnlockRange?)

(fn RotateLock)

(fn HandleTick)

(fn SetLockRotation)

(fn RotatePin
  (params (Rotation :type Float%20%28single-precision%29))
  (Transformation|SetRelativeRotation (Variables|Default|GetbobbyPin) "0, 0, 0" false false))

(fn UpdateAllowedLockRotation)

(fn SetPinOffset)