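; BP_pad is a puzzle pad in the style of Lights Out, with a highlighted state that spreads to its neighbors.
; UpdatePads toggles Highlighted on the pad and directly flips it on each entry in AdjacentPads, without cascading further.
; It also clears CanChangeMat and restores it after a two-second timer, though this Blueprint never reads that flag.
; Tick sets the Cube material every frame to match Highlighted.
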(event Custom|UpdatePads
  (Variables|Default|SetcanChangeMat? false)
  (Utilities|Time|SetTimerbyEvent (delegate Custom|CanChangeMat) 2.0)
  (Variables|Default|SetHighlighted? (not (Variables|Default|GetHighlighted?)))
  (for _array_element (Variables|Default|GetAdjacentPads)
    (if (Variables|BP_pad_C|GetHighlighted? _array_element)
      (Variables|BP_pad_C|SetHighlighted? _array_element false)
      (else
        (Variables|BP_pad_C|SetHighlighted? _array_element true)))))

(event Custom|CanChangeMat
  (Variables|Default|SetcanChangeMat? true))

(event EventTick
  (params (DeltaSeconds :type Float%20%28single-precision%29))
  (bind _cube (Variables|Default|GetCube))
  (if (Variables|Default|GetHighlighted?)
    (Rendering|Material|SetMaterial _cube 0 "/Game/Julien/Enigma/M_pad.M_pad")
    (else
      (Rendering|Material|SetMaterial _cube 0 "/Game/Julien/Enigma/M_pad2.M_pad2"))))

(fn ConstructionScript)