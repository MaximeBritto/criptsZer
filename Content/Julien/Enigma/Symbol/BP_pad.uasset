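; BP_pad is a pad in a Lights Out-style enigma puzzle, showing its highlighted state through its cube's material.
; When allowed to change, UpdatePads calls ResetPads on the EnigmaManager, then inverts its own highlight and that of each adjacent pad.
; CanUpdatePads and the pad's own ResetPads enable and disable changes.
; Tick reapplies the material matching the highlight state until HasWin is set.
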(event Custom|ResetPads
  (Variables|Default|SetcanChangeMat? false))

(event Custom|UpdatePads
  (if (Variables|Default|GetcanChangeMat?)
    (Default|ResetPads (Variables|Default|GetenigmaManager))
    (Variables|Default|SetHighlighted? (not (Variables|Default|GetHighlighted?)))
    (for _array_element (Variables|Default|GetAdjacentPads)
      (if (Variables|BP_pad_C|GetHighlighted? _array_element)
        (Variables|BP_pad_C|SetHighlighted? _array_element false)
        (else
          (Variables|BP_pad_C|SetHighlighted? _array_element true))))))

(event Custom|CanUpdatePads
  (Variables|Default|SetcanChangeMat? true))

(event EventTick
  (params (DeltaSeconds :type Float%20%28single-precision%29))
  (bind _cube (Variables|Default|GetCube))
  (if (not (Variables|Default|GethasWin?))
    (if (Variables|Default|GetHighlighted?)
      (Rendering|Material|SetMaterial _cube 0 "/Game/Julien/Enigma/Symbol/M_pad.M_pad")
      (else
        (Rendering|Material|SetMaterial _cube 0 "/Game/Julien/Enigma/Symbol/M_pad2.M_pad2")))))

(fn ConstructionScript)